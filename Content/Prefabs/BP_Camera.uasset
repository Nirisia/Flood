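; Player camera that handles zooming, rotation toggling and mouse interaction with scene objects.
; The wheel sets a clamped spring-arm length that Tick eases toward; right mouse toggles CanRotate and cursor visibility within configured view limits.
; Left click traces under the cursor, triggering water adders/removers or dragging Movable-tagged BP_DynamicMeshes.
; Dragged objects lose collision and follow a clamped Visibility trace, with a helper Plane moved to their height and position until release.
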(event EventTick
  (params (DeltaSeconds :type Float%20%28single-precision%29))
  (bind _returnvalue (Game|GetPlayerController 0))
  (bind _hitresult (Game|Player|GetHitResultUnderCursorbyChannel _returnvalue "TraceTypeQuery1" true))
  (bind _location (Collision|BreakHitResult _hitresult))
  (bind (_returnvalue_2 _returnvalue2 _returnvalue3) (|ClampLocation (.x _location) (.y _location) (.z _location)))
  ;[1 1 1] Updating object dragging
  (CallFunction|UpdateZoom)
  (Utilities|IsValid (Variables|Default|GetselectedObj)
    (:Is%20Valid
      (Transformation|SetActorLocation (Variables|Default|GetselectedObj) (Math|Vector|MakeVector _returnvalue_2 _returnvalue2 _returnvalue3) false false))))

(event EventBeginPlay
  (bind _output_get (Variables|/Script/Engine.SpringArmComponent|SetTargetArmLength (Variables|Default|GetSpringArm) 5e+02))
  (Variables|Default|SettargetZoom _output_get)
  (|Setupcamclamp))

(event Input|MouseEvents|LeftMouseButton
  (params (Key :type Key%20Structure :default "None"))
  (bind _returnvalue (Game|GetPlayerController 0))
  (bind _hitresult (Game|Player|GetHitResultUnderCursorbyChannel _returnvalue "TraceTypeQuery1" true))
  (bind _location (Collision|BreakHitResult _hitresult))
  (bind (_returnvalue_2 _returnvalue2 _returnvalue3) (|ClampLocationUnselect (.x _location) (.y _location) (.z _location)))
  ;[1 1 1] Begin/End object dragging
  (:Pressed
    (Utilities|SelectObject))
  (:Released
    (Utilities|IsValid (Variables|Default|GetselectedObj)
      (:Is%20Valid
        (|UnselectObject (Math|Vector|MakeVector _returnvalue_2 _returnvalue2 _returnvalue3))))))

(event Input|MouseEvents|MouseWheelUp
  (params (Key :type Key%20Structure :default "None"))
  ;[1 1 1] Zoom/Unzoom
  (:Pressed
    (Variables|Default|SettargetZoom (Math|Float|Clamp(Float) (- (Variables|Default|GettargetZoom) 8e+01) 1.8e+02 5.8e+02))))

(event Input|MouseEvents|MouseWheelDown
  (params (Key :type Key%20Structure :default "None"))
  ;[1 1 1] Zoom/Unzoom
  (:Pressed
    (Variables|Default|SettargetZoom (Math|Float|Clamp(Float) (+ (Variables|Default|GettargetZoom) 8e+01) 1.8e+02 5.8e+02))))

(event Input|MouseEvents|RightMouseButton
  (params (Key :type Key%20Structure :default "None"))
  (:Pressed
    (|BeginRotation))
  (:Released
    (|StopRotation)))

(fn ConstructionScript)

(fn UpdateZoom
  (bind _springarm (Variables|Default|GetSpringArm))
  (Variables|/Script/Engine.SpringArmComponent|SetTargetArmLength _springarm (Math|Float|Lerp (Variables|/Script/Engine.SpringArmComponent|GetTargetArmLength _springarm) (Variables|Default|GettargetZoom) 0.02)))