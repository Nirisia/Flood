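; Clickable window that toggles a waterfall on and off and adjusts how many spawners are adding to the linked Water.
; Each click, ignored mid-animation, switches the window's material state, increments or decrements Water.IsAdding, and plays the open or close timeline.
; The timelines pitch the mesh and drive the waterfall spline's mask parameters, re-creating its dynamic material every update.
; On finish, the waterfall's Niagara spawn rate is set and reloaded.
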(event Custom|Clicked
  (bind _waterfall (Variables|Default|GetWaterfall))
  (bind _waterfall_2 (Variables|Default|GetWaterfall))
  (bind _staticmesh (Variables|Default|GetStaticMesh))
  (bind _staticmesh_2 (Variables|Default|GetStaticMesh))
  (bind _waterfall_3 (Variables|Default|GetWaterfall))
  (bind _waterfall_4 (Variables|Default|GetWaterfall))
  (bind _returnvalue (Transformation|GetWorldRotation _staticmesh_2))
  (bind _returnvalue_2 (Transformation|GetWorldRotation _staticmesh))
  (bind _spline_mesh_component (Variables|/Game/Art/Blueprint/BP_Waterfall1.BP_Waterfall1_C|GetSpline%20Mesh%20Component _waterfall_3))
  (bind _spline_mesh_component_2 (Variables|/Game/Art/Blueprint/BP_Waterfall1.BP_Waterfall1_C|GetSpline%20Mesh%20Component _waterfall))
  (if (not (Variables|Default|GetinAnim))
    (if (Variables|Default|GetisActive)
      (Variables|Default|SetinAnim true)
      (Rendering|Material|SetScalarParameterValue (Variables|Default|GetMaterialInstance) "Window On/Off" 1.0 :!class /Script/Engine.MaterialInstanceDynamic)
      (|AddWaterSpawner)
      (bind (_direction _rotation _mask_open _mask_shutdown) (Timeline|OpenWindow PlayFromStart)
        (:Update
          (Transformation|SetWorldRotation _staticmesh_2 (Math|Rotator|MakeRotator (.roll _returnvalue) _rotation (.yaw _returnvalue)) false false)
          (bind _returnvalue_3 (Rendering|Material|CreateDynamicMaterialInstance _spline_mesh_component 0 (Rendering|Material|GetMaterial _spline_mesh_component 0) "None" :!class /Script/Engine.PrimitiveComponent))
          (Rendering|Material|SetScalarParameterValue _returnvalue_3 "Mask_Open" _mask_open :!class /Script/Engine.MaterialInstanceDynamic)
          (Rendering|Material|SetScalarParameterValue _returnvalue_3 "Mask_Shutdown" _mask_shutdown :!class /Script/Engine.MaterialInstanceDynamic)
          (Rendering|Material|SetMaterial _spline_mesh_component 0 _returnvalue_3))
        (:Finished
          (Variables|Default|SetisActive false)
          (Variables|Default|SetinAnim false)
          (Variables|/Game/Art/Blueprint/BP_Waterfall1.BP_Waterfall1_C|SetSpawnRate_Niagara _waterfall_2 2.8e+02)
          (Default|Reload _waterfall_2)))
      (else
        (Variables|Default|SetinAnim true)
        (Rendering|Material|SetScalarParameterValue (Variables|Default|GetMaterialInstance) "Window On/Off" 0.0 :!class /Script/Engine.MaterialInstanceDynamic)
        (|RemoveWaterSpawner)
        (bind (_direction_2 _rotation_2 _mask_shutdown_2) (Timeline|CloseWindow PlayFromStart)
          (:Update
            (Transformation|SetWorldRotation _staticmesh (Math|Rotator|MakeRotator (.roll _returnvalue_2) _rotation_2 (.yaw _returnvalue_2)) false false)
            (bind _returnvalue_4 (Rendering|Material|CreateDynamicMaterialInstance _spline_mesh_component_2 0 (Rendering|Material|GetMaterial _spline_mesh_component_2 0) "None" :!class /Script/Engine.PrimitiveComponent))
            (Rendering|Material|SetScalarParameterValue _returnvalue_4 "Mask_Shutdown" _mask_shutdown_2 :!class /Script/Engine.MaterialInstanceDynamic)
            (Rendering|Material|SetMaterial _spline_mesh_component_2 0 _returnvalue_4))
          (:Finished
            (Variables|Default|SetisActive true)
            (Variables|Default|SetinAnim false)
            (Variables|/Game/Art/Blueprint/BP_Waterfall1.BP_Waterfall1_C|SetSpawnRate_Niagara _waterfall_4 0.0)
            (Default|Reload _waterfall_4)))))))

(event EventBeginPlay
  (bind _staticmesh (Variables|Default|GetStaticMesh))
  (bind _returnvalue (Rendering|Material|CreateDynamicMaterialInstance _staticmesh 0 "/Game/Art/Materials/M_InteractiveObject/MI_IO_Window.MI_IO_Window" "None" :!class /Script/Engine.PrimitiveComponent))
  (bind _output_get (Variables|Default|SetMaterialInstance _returnvalue))
  (Rendering|Material|SetMaterial _staticmesh 0 _output_get))

(fn ConstructionScript)