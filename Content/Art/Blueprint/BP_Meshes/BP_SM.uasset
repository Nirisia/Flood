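; Static mesh actor that develops moss, rust and surface algae in response to the water level.
; Every tick it reads waterHeight from a parameter collection, moving moss and rust markers and animating height parameters on a dynamic mesh material.
; Rust keeps the highest level reached, while moss creeps back down after a cooldown once water drops.
; An algae plane follows the water surface, fading its gradient density through delayed timelines based on mesh-center height checks.
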(event Custom|Moss%20Disappears
  (bind _sphere_z_location (Variables|Default|GetSphere%20Z%20Location))
  (bind _mossposition (Variables|Default|GetMossPosition))
  (bind _returnvalue (Transformation|GetWorldLocation _mossposition))
  ;[1 1 1] Moss Rust Event
  ;;[1 1 1] Moss Disappears Event
  (if (< (Variables|Default|GetSphere%20Z%20Location) (.z (Variables|Default|GetSphere%20Initial%20Location)))
    (Transformation|SetWorldLocation (Variables|Default|GetMossPosition) (Variables|Default|GetSphere%20Initial%20Location) false false)
    (Variables|Default|SetMoss%20Cooldown false)
    (elif (Variables|Default|GetMoss%20Spray)
      (bind _result (Math|Float|DecrementFloat _sphere_z_location)
        (:%20%20
          (Transformation|SetWorldLocation _mossposition (Math|Vector|MakeVector (.x _returnvalue) (.y _returnvalue) _result) false false)
          (Rendering|Material|SetScalarParameterValue (Variables|Default|GetMaterialInstanceMoss) "MossHeight" _sphere_z_location :!class /Script/Engine.MaterialInstanceDynamic)
          (Variables|Default|SetMoss%20Cooldown true))))))

(event Custom|Moss%20Rust
  (bind _materialinstancemoss (Variables|Default|GetMaterialInstanceMoss))
  (bind _rustposition (Variables|Default|GetRustPosition))
  (bind _mossposition (Variables|Default|GetMossPosition))
  (bind _returnvalue (Transformation|GetWorldLocation _rustposition))
  (bind _returnvalue_2 (Transformation|GetWorldLocation _mossposition))
  ;[1 1 1] Moss Rust Event
  (Actor|GetAllActorsOfClass "/Game/Prefabs/BP_Water.BP_Water_C")
  (bind _returnvalue_3 (Rendering|Material|GetScalarParameterValue "/Game/ThirdPersonCPP/Blueprints/WaterParamCollection.WaterParamCollection" "waterHeight" :!class /Script/Engine.KismetMaterialLibrary))
  (bind _output_get (Variables|Default|SetWater%20Height _returnvalue_3))
  (Variables|Default|SetSphere%20Z%20Location (.z _returnvalue_2))
  (if (<= _output_get (.z _returnvalue_2))
    ;;[1 1 1] launch Moss Disappears Event after a few times
    (if (Variables|Default|GetMoss%20Cooldown)
      (Utilities|FlowControl|Delay 0.1)
      (CallFunction|MossDisappears)
      (else
        (Variables|Default|SetMax%20Top%20Water (Variables|Default|GetSphere%20Z%20Location))
        (if (== (Variables|Default|GetMax%20Top%20Water) (Variables|Default|GetSphere%20Z%20Location))
          (Utilities|FlowControl|Delay (Variables|Default|GetMoss%20Disappear%20CD))
          (Variables|Default|SetMoss%20Cooldown true))))
    (else
      ;;[1 1 1] Get max height each tick
      (Transformation|SetWorldLocation _mossposition (Math|Vector|MakeVector (.x _returnvalue_2) (.y _returnvalue_2) (Variables|Default|GetWater%20Height)) false false)
      (Transformation|SetWorldLocation _rustposition (Math|Vector|MakeVector (.x _returnvalue) (.y _returnvalue) (Variables|Default|GetMax%20Top%20Rust)) false false)
      (Variables|Default|SetMoss%20Cooldown false)
      (Variables|Default|SetMax%20Top%20Water (Variables|Default|GetSphere%20Z%20Location))
      (if (> (Variables|Default|GetWater%20Height) (Variables|Default|GetMax%20Top%20Rust))
        (Variables|Default|SetMax%20Top%20Rust (Variables|Default|GetWater%20Height))
        ;;[1 1 1] Apply Moss and Rust with time
        (bind _newtrack_0 (Timeline|Timeline_0 Play)
          (:Update
            (Rendering|Material|SetScalarParameterValue _materialinstancemoss "MossHeight" (Math|Float|Lerp (.z (Variables|Default|GetSphere%20Initial%20Location)) (Variables|Default|GetSphere%20Z%20Location) _newtrack_0) :!class /Script/Engine.MaterialInstanceDynamic)
            (Rendering|Material|SetScalarParameterValue _materialinstancemoss "HumidityRustHeight" (Math|Float|Lerp (.z (Variables|Default|GetSphere%20Initial%20Location)) (Variables|Default|GetMax%20Top%20Rust) _newtrack_0) :!class /Script/Engine.MaterialInstanceDynamic)
            (Variables|Default|SetMoss%20Spray false))
          (:Finished
            (Variables|Default|SetMoss%20Spray true)))
        (else
          (Timeline|Timeline_0 Play))))))

(event Custom|Algae
  (bind _algaeplane (Variables|Default|GetAlgaePlane))
  (bind _returnvalue (Transformation|GetWorldLocation _algaeplane))
  ;[1 1 1] Algae Event
  (Variables|Default|SetCube%20Z%20location (.z (Transformation|GetWorldLocation (Variables|Default|GetMeshCenter))))
  (Actor|GetAllActorsOfClass "/Game/Prefabs/BP_Water.BP_Water_C")
  (bind _returnvalue_2 (Rendering|Material|GetScalarParameterValue "/Game/ThirdPersonCPP/Blueprints/WaterParamCollection.WaterParamCollection" "waterHeight" :!class /Script/Engine.KismetMaterialLibrary))
  (bind _output_get (Variables|Default|SetWater%20Height _returnvalue_2))
  (Transformation|SetWorldLocation _algaeplane (Math|Vector|MakeVector (.x _returnvalue) (.y _returnvalue) (+ _output_get (Variables|Default|GetAlgae%20Water%20Gap))) false false)
  (Transformation|SetWorldRotation _algaeplane "0, 0, 0" false false)
  (if (Math|Boolean|Equal(Boolean) (<= (- (Variables|Default|GetCube%20Z%20location) (Variables|Default|GetCube%20Z%20location)) (Variables|Default|GetWater%20Height)) (> (+ (Variables|Default|GetCube%20Z%20location) (Variables|Default|GetCube%20Z%20location)) (Variables|Default|GetWater%20Height)))
    (Utilities|FlowControl|Delay (Variables|Default|GetCD%20Algae%20Appear))
    (if (Math|Boolean|Equal(Boolean) (<= (- (Variables|Default|GetCube%20Z%20location) (Variables|Default|GetCube%20Z%20location)) (Variables|Default|GetWater%20Height)) (> (+ (Variables|Default|GetCube%20Z%20location) (Variables|Default|GetCube%20Z%20location)) (Variables|Default|GetWater%20Height)))
      (bind _newtrack_0 (Timeline|Timeline_1 Play)
        (:Update
          (Variables|Default|SetCD%20Algae%20Disappear (Math|Float|Lerp 0.0 2.5 _newtrack_0))
          (Rendering|Material|SetScalarParameterValue (Variables|Default|GetMaterial%20Instance) "GradientDensity" (Math|Float|Lerp 0.0 2.5 _newtrack_0) :!class /Script/Engine.MaterialInstanceDynamic))))
    (elif (== (Variables|Default|GetCD%20Algae%20Disappear) 2.5)
      (Utilities|FlowControl|Delay 2.0)
      (Timeline|Timeline_1 Reverse))))

(event EventBeginPlay
  (bind _mesh (Variables|Default|GetMesh))
  (Rendering|SetVisibility (Variables|Default|GetAlgaePlane) true false)
  (Variables|Default|SetSphere%20Initial%20Location (Transformation|GetWorldLocation (Variables|Default|GetMossPosition)))
  (Variables|Default|SetMax%20Top%20Rust (Variables|Default|GetWater%20Height))
  (Variables|Default|SetCube%20Z%20location (.z (Transformation|GetWorldLocation (Variables|Default|GetMeshCenter))))
  (bind _returnvalue (Rendering|Material|CreateDynamicMaterialInstance (Variables|Default|GetAlgaePlane) 0 "/Game/Art/Materials/M_Algae/MI_Algae.MI_Algae" "None" :!class /Script/Engine.PrimitiveComponent))
  (Variables|Default|SetMaterial%20Instance _returnvalue)
  (bind _returnvalue_2 (Rendering|Material|CreateDynamicMaterialInstance _mesh 0 (Rendering|Material|GetMaterial _mesh 0) "None" :!class /Script/Engine.PrimitiveComponent))
  (bind _output_get (Variables|Default|SetMaterialInstanceMoss _returnvalue_2))
  (Rendering|Material|SetMaterial (Variables|Default|GetMesh) 0 _output_get))

(event EventTick
  (params (DeltaSeconds :type Float%20%28single-precision%29))
  (CallFunction|MossRust)
  (CallFunction|Algae))

(fn ConstructionScript)