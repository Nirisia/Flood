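; Floating mesh Blueprint that reacts to water level with buoyancy (unless being moved), moss/rust and algae.
; Tick feeds water height from a parameter collection into a dynamic moss material, created only without algae.
; The Algae event keeps a flat plane at the waterline and fades its density via delayed timeline as the mesh crosses the surface.
; Algae runs only if that moss material is valid, which BeginPlay never sets for algae meshes.
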(event Custom|Algae
  (bind _mask_size (Variables|Default|GetMask%20Size))
  (bind _algaeplane (Variables|Default|GetAlgaePlane))
  (bind _mesh (Variables|Default|GetMesh))
  (bind _returnvalue (Transformation|GetWorldLocation _mesh))
  ;[1 1 1] Algae Event
  (Variables|Default|SetCube%20Z%20location (.z (Transformation|GetWorldLocation (Variables|Default|GetMesh))))
  (Actor|GetAllActorsOfClass "/Game/Prefabs/BP_Water.BP_Water_C")
  (bind _returnvalue_2 (Rendering|Material|GetScalarParameterValue "/Game/ThirdPersonCPP/Blueprints/WaterParamCollection.WaterParamCollection" "waterHeight" :!class /Script/Engine.KismetMaterialLibrary))
  (bind _output_get (Variables|Default|SetWater%20Height _returnvalue_2))
  (Transformation|SetWorldLocation _algaeplane (Math|Vector|MakeVector (.x _returnvalue) (.y _returnvalue) (+ _output_get (Variables|Default|GetAlgae%20Water%20Gap))) false false)
  (Transformation|SetWorldRotation _algaeplane "0, 0, 0" false false)
  (if (Math|Boolean|Equal(Boolean) (<= (- (Variables|Default|GetCube%20Z%20location) _mask_size) (Variables|Default|GetWater%20Height)) (> (+ (Variables|Default|GetCube%20Z%20location) _mask_size) (Variables|Default|GetWater%20Height)))
    (Utilities|FlowControl|Delay (Variables|Default|GetCD%20Algae%20Appear))
    (if (Math|Boolean|Equal(Boolean) (<= (- (Variables|Default|GetCube%20Z%20location) _mask_size) (Variables|Default|GetWater%20Height)) (> (+ (Variables|Default|GetCube%20Z%20location) _mask_size) (Variables|Default|GetWater%20Height)))
      (bind _newtrack_0 (Timeline|Timeline_1 Play)
        (:Update
          (Variables|Default|SetCD%20Algae%20Disappear (Math|Float|Lerp 0.0 2.5 _newtrack_0))
          (Rendering|Material|SetScalarParameterValue (Variables|Default|GetMaterial%20Instance) "GradientDensity" (Math|Float|Lerp 0.0 2.5 _newtrack_0) :!class /Script/Engine.MaterialInstanceDynamic))))
    (elif (== (Variables|Default|GetCD%20Algae%20Disappear) 2.5)
      (Utilities|FlowControl|Delay 2.0)
      (Timeline|Timeline_1 Reverse))))

(event EventBeginPlay
  (bind _mesh (Variables|Default|GetMesh))
  (Rendering|SetVisibility (Variables|Default|GetAlgaePlane) true false)
  (Variables|Default|SetCube%20Z%20location (.z (Transformation|GetWorldLocation (Variables|Default|GetMesh))))
  (bind _returnvalue (Rendering|Material|CreateDynamicMaterialInstance (Variables|Default|GetAlgaePlane) 0 "/Game/Art/Materials/M_Algae/MI_Algae.MI_Algae" "None" :!class /Script/Engine.PrimitiveComponent))
  (Variables|Default|SetMaterial%20Instance _returnvalue)
  (if (not (Variables|Default|Gethas%20Algae))
    (Components|DestroyComponent (Variables|Default|GetAlgaePlane))
    (bind _returnvalue_2 (Rendering|Material|CreateDynamicMaterialInstance _mesh 0 (Rendering|Material|GetMaterial _mesh 0) "None" :!class /Script/Engine.PrimitiveComponent))
    (Utilities|IsValid _returnvalue_2
      (:Is%20Valid
        (bind _output_get (Variables|Default|SetMaterialMoss _returnvalue_2))
        (Rendering|Material|SetMaterial (Variables|Default|GetMesh) 0 _output_get)))))

(event EventTick
  (params (DeltaSeconds :type Float%20%28single-precision%29))
  (bind _materialmoss (Variables|Default|GetMaterialMoss))
  (if (Variables|Default|GetisGettingMoved)
    _
    (else
      (Class|WaterFunctionLibrary|BuoyancyCalculation (Variables|Default|GetMesh) 0.0 "ObjectTypeQuery7")))
  (bind _returnvalue (Rendering|Material|GetScalarParameterValue "/Game/ThirdPersonCPP/Blueprints/WaterParamCollection.WaterParamCollection" "waterHeight" :!class /Script/Engine.KismetMaterialLibrary))
  (Variables|Default|SetWater%20Height _returnvalue)
  (Utilities|IsValid _materialmoss
    (:Is%20Valid
      (Rendering|Material|SetScalarParameterValue _materialmoss "MossHeight" (Variables|Default|GetWater%20Height) :!class /Script/Engine.MaterialInstanceDynamic)
      (Rendering|Material|SetScalarParameterValue _materialmoss "HumidityRustHeight" (Variables|Default|GetWater%20Height) :!class /Script/Engine.MaterialInstanceDynamic)
      (if (Variables|Default|Gethas%20Algae)
        (CallFunction|Algae)))))

(fn ConstructionScript)