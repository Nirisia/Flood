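; BP_Waterfall1 is a waterfall actor that builds tapering water meshes with Niagara splash effects along a spline.
; The construction script adds a spline mesh per segment and a Niagara component at each segment's start.
; ScaleWaterfall decreases per segment, tapering mesh width and reducing splash vertical scale and spawn rate.
; Reload reapplies scale and spawn rate, but only to the last stored mesh and particle components.
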(event EventBeginPlay)

(event Collision|EventActorBeginOverlap
  (params (OtherActor :type Actor%20Object%20Reference)))

(event EventTick
  (params (DeltaSeconds :type Float%20%28single-precision%29)))

(fn ConstructionScript
  (bind _spline (Variables|Default|GetSpline))
  (bind _scale_niagara (Variables|Default|GetScale_Niagara))
  (bind (_x _y _z) (Math|Vector|BreakVector _scale_niagara))
  (for _index (range 0 (- (Spline|GetNumberOfSplinePoints (Variables|Default|GetSpline)) 2))
    (bind _returnvalue (AddComponent|AddSplineMeshComponent false (Math|Transform|MakeTransform "0, 0, 0" "0, 0, 0" (Variables|Default|GetScale))))
    (bind _output_get (Variables|Default|SetSpline%20Mesh%20Component _returnvalue))
    (Transformation|AttachComponentToComponent (Variables|Default|GetSpline%20Mesh%20Component) 0 "None" "KeepRelative" "KeepRelative" "KeepRelative" true)
    (bind _returnvalue_2 (AddComponent|AddNiagaraComponent false (Math|Conversions|ToTransform(Vector) (.Location (Spline|GetLocationandTangentatSplinePoint _spline _index "Local")))))
    (Variables|Default|SetParticle _returnvalue_2)
    (SplineMesh|SetForwardAxis _output_get "Z" true)
    (SplineMesh|SetStartandEnd _output_get (.Location (Spline|GetLocationandTangentatSplinePoint _spline _index "Local")) (.Tangent (Spline|GetLocationandTangentatSplinePoint _spline _index "Local")) (.Location (Spline|GetLocationandTangentatSplinePoint _spline (+ _index 1) "Local")) (.Tangent (Spline|GetLocationandTangentatSplinePoint _spline (+ _index 1) "Local")) true :!class /Script/Engine.SplineMeshComponent)
    (SplineMesh|SetStartScale (Variables|Default|GetSpline%20Mesh%20Component) (Math|Vector2D|MakeVector2D (Variables|Default|GetScale_Waterfall) (Variables|Default|GetScale_Waterfall)) true :!class /Script/Engine.SplineMeshComponent)
    (Niagara|SetNiagaraVariable(Vector3) _returnvalue_2 "Scale_Splash" (Math|Vector|MakeVector _x _y (* _z (Variables|Default|GetScale_Waterfall))))
    (Niagara|SetNiagaraVariable(Float) _returnvalue_2 "SpawnRate_Splash" (* (Variables|Default|GetSpawnRate_Niagara) (Variables|Default|GetScale_Waterfall)))
    (Variables|Default|SetScale_Waterfall (- (Variables|Default|GetScale_Waterfall) (/ 1.0 (Math|Conversions|ToFloat(Integer) (Spline|GetNumberOfSplinePoints (Variables|Default|GetSpline))))))
    (SplineMesh|SetEndScale (Variables|Default|GetSpline%20Mesh%20Component) (Math|Vector2D|MakeVector2D (Variables|Default|GetScale_Waterfall) (Variables|Default|GetScale_Waterfall)) true :!class /Script/Engine.SplineMeshComponent)))

(fn Reload
  (for _index (range 0 (- (Spline|GetNumberOfSplinePoints (Variables|Default|GetSpline)) 2))
    (Transformation|SetRelativeScale3D (Variables|Default|GetSpline%20Mesh%20Component) (Variables|Default|GetScale))
    (Niagara|SetNiagaraVariable(Float) (Variables|Default|GetParticle) "SpawnRate_Splash" (* (Variables|Default|GetSpawnRate_Niagara) (Variables|Default|GetScale_Waterfall)))))