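; Procedural plant Blueprint that builds a tapering stem along an editable spline in the Construction Script.
; Each segment gets a Z-forward spline mesh bent between neighboring points, plus two more spline mesh components placed at its end points and oriented to the tangent.
; ScalePlant and Scale are recomputed per segment from Growth and point count, so thickness changes cumulatively along the spline.
; The event graph is empty, so nothing animates growth at runtime.
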(event EventBeginPlay)

(event Collision|EventActorBeginOverlap
  (params (OtherActor :type Actor%20Object%20Reference)))

(event EventTick
  (params (DeltaSeconds :type Float%20%28single-precision%29)))

(fn ConstructionScript
  (bind _spline (Variables|Default|GetSpline))
  (bind _growth (Variables|Default|GetGrowth))
  (for _index (range 0 (- (Spline|GetNumberOfSplinePoints _spline) 2))
    (bind _returnvalue (AddComponent|AddSplineMeshComponent false))
    (bind _output_get (Variables|Default|SetSpline%20Mesh%20Component _returnvalue))
    (Transformation|AttachComponentToComponent _output_get 0 "None" "KeepRelative" "KeepRelative" "KeepRelative" true)
    (SplineMesh|SetForwardAxis _returnvalue "Z" true)
    (SplineMesh|SetStartandEnd _returnvalue (.Location (Spline|GetLocationandTangentatSplinePoint _spline _index "Local")) (.Tangent (Spline|GetLocationandTangentatSplinePoint _spline _index "Local")) (.Location (Spline|GetLocationandTangentatSplinePoint _spline (+ _index 1) "Local")) (.Tangent (Spline|GetLocationandTangentatSplinePoint _spline (+ _index 1) "Local")) true :!class /Script/Engine.SplineMeshComponent)
    (AddComponent|AddSplineMeshComponent false (Math|Transform|MakeTransform (.Location (Spline|GetLocationandTangentatSplinePoint _spline (+ _index 1) "Local")) (Math|Conversions|RotationFromXVector (.Tangent (Spline|GetLocationandTangentatSplinePoint _spline (+ _index 1) "Local"))) (Variables|Default|GetScale)))
    (bind _returnvalue_2 (AddComponent|AddSplineMeshComponent false (Math|Transform|MakeTransform (.Location (Spline|GetLocationandTangentatSplinePoint (Variables|Default|GetSpline) _index "Local")) (Math|Conversions|RotationFromXVector (.Tangent (Spline|GetLocationandTangentatSplinePoint (Variables|Default|GetSpline) _index "Local"))) "0.050000,1.500000,1.500000")))
    (SplineMesh|SetStartScale _returnvalue_2 (Math|Vector2D|MakeVector2D (Variables|Default|GetScale_Plant) (Variables|Default|GetScale_Plant)) true :!class /Script/Engine.SplineMeshComponent)
    (SplineMesh|SetStartScale _returnvalue (Math|Vector2D|MakeVector2D (Variables|Default|GetScale_Plant) (Variables|Default|GetScale_Plant)) true :!class /Script/Engine.SplineMeshComponent)
    (Variables|Default|SetScale_Plant (Math|Float|Clamp(Float) (* _growth (- (Variables|Default|GetScale_Plant) (/ 1.0 (Math|Conversions|ToFloat(Integer) (Spline|GetNumberOfSplinePoints (Variables|Default|GetSpline)))))) 0.0 2e+01))
    (Variables|Default|SetScale (Math|Vector|ClampVectorSize (* (Math|Vector|MakeVector (* 0.3 (Math|Float|Clamp(Float) (- (Variables|Default|GetScale_Plant) (/ 1.0 (Math|Conversions|ToFloat(Integer) (Spline|GetNumberOfSplinePoints (Variables|Default|GetSpline))))) 0.0 2e+02)) (Math|Float|Clamp(Float) (- (Variables|Default|GetScale_Plant) (/ 1.0 (Math|Conversions|ToFloat(Integer) (Spline|GetNumberOfSplinePoints (Variables|Default|GetSpline))))) 0.0 2e+02) (Math|Float|Clamp(Float) (- (Variables|Default|GetScale_Plant) (/ 1.0 (Math|Conversions|ToFloat(Integer) (Spline|GetNumberOfSplinePoints (Variables|Default|GetSpline))))) 0.0 2e+02)) _growth) 0.0 2e+01))
    (SplineMesh|SetEndScale _returnvalue_2 (Math|Vector2D|MakeVector2D (Variables|Default|GetScale_Plant) (Variables|Default|GetScale_Plant)) true :!class /Script/Engine.SplineMeshComponent)
    (SplineMesh|SetEndScale _returnvalue (Math|Vector2D|MakeVector2D (Variables|Default|GetScale_Plant) (Variables|Default|GetScale_Plant)) true :!class /Script/Engine.SplineMeshComponent)))