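; BP_WaterComponent is a component that makes its owning actor disturb interactive water surfaces beneath it.
; Every tick it line-traces straight down from the bottom center of the owner's bounds over TraceDistance, against a single object type.
; When the hit actor is a WaterSurface_BP, it stores it and calls ApplyLocalSplat at the owner's location, sized by ImpacteSize.
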(event EventBeginPlay)

(event EventTick
  (params (DeltaSeconds :type Float%20%28single-precision%29))
  (bind _returnvalue (Components|GetOwner))
  (bind (_origin _boxextent) (Collision|GetActorBounds _returnvalue false false))
  (bind _returnvalue_2 (- (.z _origin) (.z _boxextent)))
  (bind _returnvalue_3 (Math|Vector|MakeVector (.x _origin) (.y _origin) _returnvalue_2))
  (Utilities|IsValid _returnvalue
    (:Is%20Valid
      (bind _outhit (Collision|LineTraceForObjects _returnvalue_3 (+ _returnvalue_3 (* "0, 0,-1.000000" (Variables|Default|GetTraceDistance))) (Utilities|Array|MakeArray "ObjectTypeQuery7") false 0 "None"))
      (Variables|Default|SetHit _outhit)
      (bind _aswater_surface_bp (Utilities|Casting|CastToWaterSurface_BP (.HitActor (Collision|BreakHitResult (Variables|Default|GetHit)))))
      (Variables|Default|SetInteractiveWater _aswater_surface_bp)
      (Default|ApplyLocalSplat (Variables|Default|GetInteractiveWater) (Transformation|GetActorLocation (Components|GetOwner)) (Variables|Default|GetImpacteSize)))))